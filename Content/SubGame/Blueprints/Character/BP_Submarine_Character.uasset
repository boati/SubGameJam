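; BP_Submarine_Character is the player submarine, driven by movement axes and aimed by thumbstick or mouse.
; Forward and right inputs move it along fixed world X and Y, independent of facing.
; Thumbstick input outside the dead zone rotates the actor and sets UsingController, which is never cleared here.
; Until then, Tick sets yaw from the BP_SubController mouse deprojection direction, printing a GameMode error if the cast fails.
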(event `InputAxis|MoveRight`
  (params (AxisValue :type "Float (single-precision)"))
  (`self.AddMovementInput` (0.0 1.0 0.0) AxisValue))

(event `InputAxis|MoveForward`
  (params (AxisValue :type "Float (single-precision)"))
  (`self.AddMovementInput` (1.0 0.0 0.0) AxisValue))

(event `InputAxis|ThumbStick X`
  (params (AxisValue :type "Float (single-precision)"))
  (bind _returnvalue (`KismetMathLibrary.MakeVector` (stale `InputAxis|ThumbStick Y` AxisValue) AxisValue))
  (if (!= _returnvalue (0.0 0.0 0.0) :`ErrorTolerance` (`self.DeadZone`)) :!label _label
    (set `self.bUsingController` true)
    (`self.SetActorRotation` (`KismetMathLibrary.MakeRotFromX` _returnvalue))))

(event `InputAxis|ThumbStick Y`
  (params (AxisValue :type "Float (single-precision)"))
  (goto _label))

(event `self.ReceiveTick`
  (params (DeltaSeconds :type "Float (single-precision)"))
  (bind _asbp_sub_controller (cast `/Game/SubGame/Blueprints/GameMode/Controller/BP_SubController` (`self.GetController`))
    (:`then`
      ;[1 1 1] This is how we check if we're using mouse input!
      (if (not (`self.bUsingController`))
        (bind (_returnvalue_roll _returnvalue_pitch _returnvalue_yaw) (`KismetMathLibrary.BreakRotator` (`KismetMathLibrary.MakeRotFromX` (`.WorldDirection` (`PlayerController.DeprojectMousePositionToWorld` _asbp_sub_controller)))))
        ;[1 1 1] Get the mouse position in 3d space, then turn the ship to look at
        (`self.SetActorRotation` (`KismetMathLibrary.MakeRotator` 0.0 0.0 _returnvalue_yaw))))
    (:`CastFailed`
      (`KismetSystemLibrary.PrintString` "Improper GameMode Settings!") ; This shouldn't be reached.
    )))

(fn `UserConstructionScript`)